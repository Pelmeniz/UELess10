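; BP_Bonus is an Arcanoid bonus actor that carries one of three randomly chosen bonus types and travels through the level.
; The construction script rolls the type and writes its enum name to a TextRender as a label.
; Each Tick moves it by Direction and Speed with a swept offset, destroying it on any blocking hit.
; No pickup or bonus effect is implemented in this graph.
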(event `self.ReceiveTick`
  (params (DeltaSeconds :type "Float (single-precision)"))
  (bind _sweephitresult (`self.K2_AddActorWorldOffset` (* (* (`self.Direction`) (`self.Speed`)) DeltaSeconds) true))
  (if (`GameplayStatics.BreakHitResult` _sweephitresult)
    (`self.K2_DestroyActor`)))

(fn `UserConstructionScript`
  (set `self.BonusType` (select `int` (`KismetMathLibrary.RandomIntegerInRange` 0 2) :`0` "NewEnumerator0" :`1` "NewEnumerator1" :`2` "NewEnumerator2" :!type "/Game/Arcanoid/Blueprints/Bonuses/E_Bonus_Type Enum"))
  (`TextRenderComponent.K2_SetText` (`self.TextRender`) (`KismetTextLibrary.Conv_StringToText` (`|GetEnumeratorNameAsString` (`self.BonusType`)))))