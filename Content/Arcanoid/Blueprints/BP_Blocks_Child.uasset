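; BP_Blocks_Child is an Arkanoid block variant that can drop a bonus when destroyed.
; On BeginPlay a random bool decides whether the block binds SpawnBonus to its own OnDestroyed event.
; SpawnBonus spawns a BP_Bonus at the block's location with a fixed rotation.
; The construction script only calls the parent's, and Tick and overlap events are disabled stubs.
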(event `self.ReceiveBeginPlay`
  ;[1 0.3162 0.2465] Рандомная активация бонуса
  (if (`KismetMathLibrary.RandomBool`)
    (add `self.OnDestroyed` (delegate `SpawnBonus`))))

(event `SpawnBonus` :!signature `self.OnDestroyed`
  (params (DestroyedActor :type "Actor Object Reference"))
  ;[1 0.3162 0.2465] Рандомная активация бонуса
  (`|SpawnActorFromClass` "/Game/Arcanoid/Blueprints/Bonuses/BP_Bonus.BP_Bonus_C" (`KismetMathLibrary.MakeTransform` (`self.K2_GetActorLocation`) (struct :`Pitch` -90.0)) "Undefined" "OverrideRootScale" null null))

(fn `UserConstructionScript`
  (`parent.UserConstructionScript`))