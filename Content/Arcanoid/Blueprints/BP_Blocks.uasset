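; BP_Blocks is a breakable block for an Arkanoid game that loses a life each time the ball hits it.
; The Cube's hit event filters for BP_Ball through a cast and calls the BallHit event, which decrements Lives.
; At zero or below the block destroys itself; otherwise SetMaterial switches on Lives, with only the one-life case defined, turning the cube green.
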(event `self.ReceiveBeginPlay`)

(event `self.Cube.OnComponentHit`
  (params (HitComponent :type "PrimitiveComponent Object Reference") (OtherActor :type "Actor Object Reference") (OtherComp :type "PrimitiveComponent Object Reference") (NormalImpulse :type "Vector Structure") (Hit :type "HitResult Structure (by ref)"))
  ;[0.256 1 0.4491] Проверка на касание с шариком и запуск ивента
  (cast `/Game/Arcanoid/Blueprints/BP_Ball` OtherActor)
  (`self.BallHit`))

(event `BallHit`
  ;[0.973 1 0.4503] Запуск ивента при касании шарика на смену материала или уничтожение актора
  (bind _result (`/Engine/EditorBlueprintResources/StandardMacros.DecrementInt` (`self.Lives`))
    (:`  `
      (if (<= _result 0)
        (`self.K2_DestroyActor`)
        (else
          (`self.SetMaterial`))))))

(fn `SetMaterial`
  ;[1 0.4999 0.5098] Функция смены материала
  (bind _output_get (set `self.Lives` (`self.Lives`)))
  (switch `int` _output_get
    (:`1`
      (`PrimitiveComponent.SetMaterial` (`self.Cube`) 0 "/Game/Arcanoid/Materials/M_Color_Green.M_Color_Green"))))

(fn `UserConstructionScript`)