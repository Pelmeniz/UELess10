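; BP_MyPlayerController is the player controller for an Arcanoid game, turning horizontal input into movement of the player's pawn.
; On possess it casts the pawn to BP_MyPawn and stores it, and on BeginPlay it switches input to game-only mode.
; The Left_Right axis offsets the stored pawn along world Y, scaled by speed and delta time, with sweep enabled for collision.
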(event `self.ReceivePossess`
  (params (PossessedPawn :type "Pawn Object Reference"))
  ;[0.3521 1 0.4223] Управление пешкой
  (bind _asbp_my_pawn (cast `/Game/Arcanoid/Blueprints/Core/BP_MyPawn` PossessedPawn))
  (set `self.MyPawn` _asbp_my_pawn))

(event `self.ReceiveBeginPlay`
  ;[1 0.3236 0.4335] Автоматическая активация игры
  (`WidgetBlueprintLibrary.SetInputMode_GameOnly` self))

(event `InputAxis|Left_Right`
  (params (AxisValue :type "Float (single-precision)"))
  (`self.K2_AddActorWorldOffset` (`self.MyPawn`) (`KismetMathLibrary.MakeVector` 0.0 (* AxisValue (`GameplayStatics.GetWorldDeltaSeconds`) (`self.Speed`))) true false))

(fn `UserConstructionScript`)