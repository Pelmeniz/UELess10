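; BP_BlocksGenerator is an Arkanoid block generator that lays out a grid of blocks with an editor preview.
; The Construction Script adds a static mesh component per grid cell from X, Y and Padding, storing each in PrewiewArray.
; On BeginPlay it destroys those preview components and spawns BP_Blocks_Child actors at the same offsets from its location.
; Spawn offsets follow world axes, so actor rotation and scale are ignored, unlike the relative preview.
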(event `self.ReceiveBeginPlay`
  (bind (_returnvalue_x _returnvalue_y _returnvalue_z) (`KismetMathLibrary.BreakVector` (`self.K2_GetActorLocation`)))
  ;[0.2154 1 0.9303] Вытягивание и уничтожение компонентов из превью
  (for _array_element (`self.PrewiewArray`)
    (`ActorComponent.K2_DestroyComponent` _array_element))
  ;[1 0.4792 0.9404] Создание блоков на основе превью сетки
  (for _index (range (+ (`self.X`) 1))
    (for _index_2 (range (+ (`self.Y`) 1))
      (`|SpawnActorFromClass` "/Game/Arcanoid/Blueprints/BP_Blocks_Child.BP_Blocks_Child_C" (`KismetMathLibrary.MakeTransform` (`KismetMathLibrary.MakeVector` (+ _returnvalue_x (`KismetMathLibrary.Conv_IntToDouble` (* _index (`self.Padding`)))) (+ _returnvalue_y (`KismetMathLibrary.Conv_IntToDouble` (* _index_2 (`self.Padding`)))) _returnvalue_z)) "Undefined" "OverrideRootScale" null null))))

(fn `UserConstructionScript`
  ;[1 0.5645 0.4441] Создание массивов блоков для превью
  (for _index (range (+ (`self.X`) 1))
    (for _index_2 (range (+ (`self.Y`) 1))
      (bind _returnvalue (`AddComponent|NODE_AddStaticMeshComponent-0` :`RelativeTransform` (`KismetMathLibrary.MakeTransform` (`KismetMathLibrary.MakeVector` (`KismetMathLibrary.Conv_IntToDouble` (* _index (`self.Padding`))) (`KismetMathLibrary.Conv_IntToDouble` (* _index_2 (`self.Padding`)))))))
      (`KismetArrayLibrary.Array_Add` (`self.PrewiewArray`) _returnvalue))))